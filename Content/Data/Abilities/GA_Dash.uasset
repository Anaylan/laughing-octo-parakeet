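; GA_Dash is a Gameplay Ability that performs a dash for the playable character by playing a direction-based animation montage.
; On activation it commits, gets the montage from the character's GetMontageByDirection and plays it through a montage-and-wait task.
; The ability ends on any montage outcome, the GameplayCue.FinishedAnimation event, or a failed character cast.
; On end, it stops the montage if the character is moving.
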(event Ability|EventActivateAbility
  (Ability|CommitAbility)
  (bind _asbp_playable_character (Utilities|Casting|CastToBP_PlayableCharacter (.OwnerActor (Utilities|Struct|BreakGameplayAbilityActorInfo (Ability|GetActorInfo))))
    (:then
      (bind _output_get (Variables|Default|SetCurMontage (Class|BaseCharacter|GetMontagebyDirection _asbp_playable_character (Variables|Default|GetActionBlend))))
      (|PlayMontageandWaitProxy "None" _output_get 1.0 "None" true 1.0 0.0 "(TagName=\"GameplayCue.FinishedAnimation\")"
        (:OnCompleted
          _)
        (:OnBlendOut
          _)
        (:OnInterrupted
          _)
        (:OnCancelled
          _)
        (:EventReceived
          _)))
    (:CastFailed
      _))
  (Ability|EndAbility))

(event Ability|EventOnEndAbility
  (params (bWasCancelled :type Boolean))
  (bind _asbp_playable_character (Utilities|Casting|CastToBP_PlayableCharacter (.OwnerActor (Utilities|Struct|BreakGameplayAbilityActorInfo (Ability|GetActorInfo)))))
  (if (Class|BaseCharacter|IsMoving _asbp_playable_character)
    (Animation|StopAnimMontage _asbp_playable_character (Variables|Default|GetCurMontage))))