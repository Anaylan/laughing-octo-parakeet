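; BP_PlayableCharacter is a character Blueprint for playable characters, adding movement debug drawing and a simple health-to-death reaction.
; Each tick, if DebugComponent is valid, it draws color-coded, height-staggered arrows for control rotation, target velocity direction and velocity direction.
; When health changes, it prints the current value on screen and calls OnDeath if the character is no longer alive.
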(event EventBeginPlay)

(event Collision|EventActorBeginOverlap
  (params (OtherActor :type Actor%20Object%20Reference)))

(event EventTick
  (params (DeltaSeconds :type Float%20%28single-precision%29))
  (bind _debugcomponent (Variables|Default|GetDebugComponent))
  (Utilities|IsValid _debugcomponent
    (:Is%20Valid
      (Class|DebugComponent|DrawControlRotation _debugcomponent 1e+02 "(R=0.040371,G=0.614583,B=0.048546,A=1.000000)" 6.0 0.0)
      (Class|DebugComponent|DrawTargetVelocityDirection _debugcomponent 1e+02 "(R=0.157541,G=0.000000,B=0.796875,A=1.000000)" 6.0 6.0)
      (Class|DebugComponent|DrawVelocityDirection _debugcomponent 1e+02 "(R=1.000000,G=0.037429,B=0.000000,A=1.000000)" 6.0 12.0))))

(event EventOnHealthChanged
  (params (Delta :type Float%20%28single-precision%29) (EventTags :type Gameplay%20Tag%20Container%20Structure%20%28by%20ref%29))
  (bind _returnvalue (Class|BaseCharacter|GetHealth))
  (Development|PrintString (Utilities|String|ToString(Float) _returnvalue) true false)
  (if (not (Class|BaseCharacter|IsAlive))
    (Class|BaseCharacter|OnDeath)))

(fn ConstructionScript)